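; ARSceneRoot_BP is an AR scene actor that animates a skeletal building mesh toward a progress value set from the HUD.
; It binds to the main HUD widget's progress-changed event and starts moving toward full progress on BeginPlay.
; Each new target restarts a timed blend whose duration scales with distance over a base speed.
; Tick eases the value through a float curve and writes it into the mesh's AnimBlueprint.
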(event `self.ReceiveBeginPlay`
  (bind _asmain_hud (cast `/Game/Blueprints/UI/MainHUD` (`PlayerController.GetHUD` (`GameplayStatics.GetPlayerController` 0))))
  (add `/Game/Blueprints/UI/MainWidget.OnProgressChanged` (`/Game/Blueprints/UI/MainHUD.MainWidget` _asmain_hud) (delegate `OnProgressChanged`))
  (`self.SetTargetProgress` 1.0))

(event `OnProgressChanged`
  (params (NewProgress :type "Float (double-precision)"))
  (`self.SetTargetProgress` NewProgress))

(event `self.ReceiveActorBeginOverlap`
  (params (OtherActor :type "Actor Object Reference")))

(event `self.ReceiveTick`
  (params (DeltaSeconds :type "Float (single-precision)"))
  (if (> (`self.MoveTime`) (`self.TimePassed`))
    (set `self.TimePassed` (`KismetMathLibrary.FClamp` (+ (`self.TimePassed`) DeltaSeconds) 0.0 (`self.MoveTime`)))
    (bind _output_get (set `self.CurrentProgress` (`KismetMathLibrary.Lerp` (`self.InitialProgress`) (`self.TargetProgress`) (`CurveFloat.GetFloatValue` (`self.SmoothLerp`) (/ (`self.TimePassed`) (`self.MoveTime`))))))
    (bind _astest_ue_09_skeleton_anim_blueprint (cast `/Game/Models/test_ue_09_Skeleton_AnimBlueprint` (`SkeletalMeshComponent.GetAnimInstance` (`SkeletalMeshActor.SkeletalMeshComponent` (`self.BuildingMesh`)))))
    (set `/Game/Models/test_ue_09_Skeleton_AnimBlueprint.Progress` _output_get _astest_ue_09_skeleton_anim_blueprint)))

(fn `SetTargetProgress`
  (params (TargetProgress :type "Float (double-precision)"))
  (set `self.TargetProgress` TargetProgress)
  (set `self.InitialProgress` (`self.CurrentProgress`))
  (set `self.MoveTime` (/ (`KismetMathLibrary.Abs` (- (`self.TargetProgress`) (`self.InitialProgress`))) (`self.BaseSpeed`)))
  (set `self.TimePassed` 0.0))

(fn `UserConstructionScript`)