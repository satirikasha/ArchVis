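; AR actor, with a bike-material mesh, that can be rotated and scaled by touch.
; Touch on the mesh records starting transform and finger position; Tick maps horizontal drag to yaw and vertical drag to uniform scale.
; BeginPlay feeds the ARToolkit camera frame and resolution into a dynamic material on Cube, serving as shadow receiver.
; ChangeColor applies a given texture to the mesh through a dynamic Bike material.
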(event `self.StaticMesh.OnInputTouchBegin`
  (params (FingerIndex :type "ETouchIndex Enum" :default "Touch1") (TouchedComponent :type "PrimitiveComponent Object Reference"))
  (bind _staticmesh (`self.StaticMesh`))
  (bind (_locationx _locationy _biscurrentlypressed) (`PlayerController.GetInputTouchState` (`GameplayStatics.GetPlayerController` 0) "Touch1"))
  ;[1 1 1] Rotation with TOUCH
  (set `self.IsPressed` true)
  (set `self.RotationStart` (`SceneComponent.RelativeRotation` _staticmesh))
  (set `self.ScaleStart` (`SceneComponent.RelativeScale3D` _staticmesh))
  (set `self.MouseXStart` _locationx)
  (set `self.MouseYStart` _locationy))

(event `self.ReceiveTick`
  (params (DeltaSeconds :type "Float (single-precision)"))
  (bind _staticmesh (`self.StaticMesh`))
  (bind (_locationx _locationy _biscurrentlypressed) (`PlayerController.GetInputTouchState` (`GameplayStatics.GetPlayerController` 0) "Touch1"))
  (bind _returnvalue (/ (- _locationy (`self.MouseYStart`)) 100.0))
  ;[1 1 1] Rotation with TOUCH
  (if _biscurrentlypressed
    (if (`self.IsPressed`)
      (`SceneComponent.K2_SetRelativeRotation` _staticmesh (`KismetMathLibrary.ComposeRotators` (`KismetMathLibrary.MakeRotator` 0.0 0.0 (- _locationx (`self.MouseXStart`))) (`self.RotationStart`)) false false)
      (`SceneComponent.SetRelativeScale3D` _staticmesh (+ (`self.ScaleStart`) (`KismetMathLibrary.MakeVector` _returnvalue _returnvalue _returnvalue))))
    (else
      (set `self.IsPressed` _biscurrentlypressed))))

(event `self.ReceiveBeginPlay`
  ;[1 1 1] Set camera resolution for shadow receiver texture
  (bind _returnvalue (`ARToolkitComponent.GetCameraFrame`))
  (bind _returnvalue_2 (`ARToolkitComponent.CreateDynamicMaterialInstance` (`self.Cube`) "/Game/Materials/BaseFeedScreen.BaseFeedScreen"))
  (`ARToolkitComponent.SetTextureParameterValue` _returnvalue_2 _returnvalue "Color")
  (bind (_webcamresx _webcamresy) (`ARToolkitComponent.GetCameraResolution` (`self.ARToolkit`)))
  (`MaterialInstanceDynamic.SetScalarParameterValue` _returnvalue_2 "CamResX" (`KismetMathLibrary.Conv_IntToDouble` _webcamresx))
  (`MaterialInstanceDynamic.SetScalarParameterValue` _returnvalue_2 "CamResY" (`KismetMathLibrary.Conv_IntToDouble` _webcamresy)))

(fn `ChangeColor`
  (params (Texture :type "Texture2D Object Reference"))
  (bind _returnvalue (`PrimitiveComponent.CreateDynamicMaterialInstance` (`self.StaticMesh`) 0 "/Game/HarleyDavidson/bike.bike"))
  (`MaterialInstanceDynamic.SetTextureParameterValue` _returnvalue "Texture" Texture))

(fn `UserConstructionScript`)